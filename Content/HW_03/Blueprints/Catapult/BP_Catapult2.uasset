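; BP_Catapult2 is a physics-driven catapult whose Spoon is aligned to the actor's rotation on BeginPlay.
; Its Fire event swings the arm by spiking the PhysicsConstraint's angular drive strength, then drops it low after a delay.
; After a second delay it spawns a BP_Cannonball at a fixed world-space offset from the Spoon as a reload and sets a moderate drive strength.
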(event `self.ReceiveBeginPlay`
  (`SceneComponent.K2_SetWorldRotation` (`self.Spoon`) (`KismetMathLibrary.TransformRotation` (`self.GetTransform`)) false false))

(event `/Game/ThirdPerson/Blueprints/BPI_Interract.Fire`
  (bind _spoon (`self.Spoon`))
  (bind _returnvalue (`PhysicsConstraintComponent.GetConstraint` (`self.PhysicsConstraint`)))
  (`ConstraintInstanceBlueprintLibrary.SetAngularDriveParams` _returnvalue 5000.0)
  (`KismetSystemLibrary.Delay` 1.0)
  (`ConstraintInstanceBlueprintLibrary.SetAngularDriveParams` _returnvalue 13.0)
  (`KismetSystemLibrary.Delay` 2.0)
  (`|SpawnActorFromClass` "/Game/HW_03/Blueprints/Cannonball/BP_Cannonball.BP_Cannonball_C" (`KismetMathLibrary.MakeTransform` (+ (`SceneComponent.K2_GetComponentLocation` _spoon) (0.0 -330.0 170.0)) (`SceneComponent.K2_GetComponentRotation` _spoon)) "Undefined" "MultiplyWithRoot" null null)
  (`ConstraintInstanceBlueprintLibrary.SetAngularDriveParams` _returnvalue 50.0))

(fn `UserConstructionScript`)